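; BP_TobyTrigger is a trigger volume actor that awards the ACH_Toby achievement when enough tagged actors are inside it at once.
; Overlap begin and end events keep a running count of actors carrying ValidActorTag.
; Each valid entry runs CheckCompleted, which compares the count to Required, awards the achievement through the FIL game instance and destroys the trigger.
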(event OnComponentBeginOverlap(Trigger)
  (params (OverlappedComponent :type Primitive%20Component%20Object%20Reference) (OtherActor :type Actor%20Object%20Reference) (OtherComp :type Primitive%20Component%20Object%20Reference) (OtherBodyIndex :type Integer) (bFromSweep :type Boolean) (SweepResult :type Hit%20Result%20Structure%20%28by%20ref%29))
  (if (Actor|ActorHasTag OtherActor (Variables|Default|GetValidActorTag))
    (Math|Integer|IncrementInt (Variables|Default|GetAmountInside)
      (:%20%20
        (CallFunction|CheckCompleted)))))

(event OnComponentEndOverlap(Trigger)
  (params (OverlappedComponent :type Primitive%20Component%20Object%20Reference) (OtherActor :type Actor%20Object%20Reference) (OtherComp :type Primitive%20Component%20Object%20Reference) (OtherBodyIndex :type Integer))
  (if (Actor|ActorHasTag OtherActor (Variables|Default|GetValidActorTag))
    (Math|Integer|DecrementInt (Variables|Default|GetAmountInside))))

(fn ConstructionScript)

(fn CheckCompleted
  (if (>= (Variables|Default|GetAmountInside) (Variables|Default|GetRequired))
    (Default|AwardAchievementfromName (Utilities|GetFILGameInstance) "ACH_Toby")
    (Actor|DestroyActor)))