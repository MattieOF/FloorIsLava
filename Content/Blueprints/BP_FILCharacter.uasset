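; Player character for a lava-hazard game that handles death on BP_Lava floors and respawn at its BeginPlay location.
; Tick checks the movement component's floor actor and calls PlayerDie, which spawns BP_Burned, hides the character, disables input and freezes the view on a temporary camera actor.
; If the game mode's DecrementLives succeeds, BeginRespawn restores the character after a delay and blends the view back.
; A leftover debug F key zeroes lives and kills the player.
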(event Custom|BeginRespawn
  (Utilities|FlowControl|Delay 1.4)
  (Transformation|SetActorLocation (Variables|Default|GetSpawnPosition) false false)
  (Rendering|SetActorHiddenInGame false)
  (Variables|Default|SetAlive true)
  (Game|Player|SetViewTargetwithBlend (Game|GetPlayerController 0) (.Character (Utilities|GetFILCharacter)) 0.75 "VTBlend_Linear" 0.0 false)
  (Utilities|FlowControl|Delay 0.75)
  (Input|EnableInput (Game|GetPlayerCharacter 0) (Game|GetPlayerController 0))
  (Actor|DestroyActor (Variables|Default|GetDeathCam)))

(event EventTick
  (params (DeltaSeconds :type Float%20%28single-precision%29))
  ;[1 1 1] On tick: check for player standing on lava
  (if (== (Utilities|GetClass (.hitactor (.hitresult (Variables|/Script/Engine.CharacterMovementComponent|GetCurrentFloor (Variables|Character|GetCharacterMovement))))) "/Game/Blueprints/BP_Lava.BP_Lava_C")
    (CallFunction|PlayerDie)))

(event EventBeginPlay
  ;[1 1 1] Init spawn position
  (Variables|Default|SetSpawnPosition (Transformation|GetActorLocation)))

(event Input|KeyboardEvents|F
  (params (Key :type Key%20Structure :default "None"))
  ;[1 0 0 1 30] Debug stuff, REMOVE THIS LOL
  (:Pressed
    (Variables|/Game/Blueprints/GI_FloorIsLava.GI_FloorIsLava_C|SetLives (Utilities|GetFILGameInstance) 0)
    (CallFunction|PlayerDie)))

(fn ConstructionScript
  (|CallParentFunction))

(fn PlayerDie
  (if (Variables|Default|GetAlive)
    (Game|SpawnActorfromClass "/Game/Particles/BP_Burned.BP_Burned_C" (Transformation|GetWorldTransform (Variables|Character|GetMesh)) "Undefined" 0 0)
    (Rendering|SetActorHiddenInGame true)
    (Variables|Default|SetAlive false)
    (bind _returnvalue (Game|SpawnActorfromClass "/Game/Blueprints/BP_Empty.BP_Empty_C" (Transformation|GetWorldTransform (Variables|Default|GetFollowCamera)) "Undefined" 0 0))
    (Game|Player|SetViewTargetwithBlend (Game|GetPlayerController 0) _returnvalue 0.0 "VTBlend_Linear" 0.0 false)
    (Variables|Default|SetDeathCam _returnvalue)
    (Input|DisableInput (Game|GetPlayerCharacter 0) (Game|GetPlayerController 0))
    (bind _shouldrespawn (Default|DecrementLives (.GameMode (Utilities|GetFILGameMode))))
    (if _shouldrespawn
      (CallFunction|BeginRespawn))))