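; Game mode for the FIL game that runs each level's opening and moves between levels through the game instance's level list.
; BeginPlay records the level reached, views an OpeningCam-tagged actor with input disabled, and shows the level name or, before the game has started, an achievements menu.
; StartLevel blends to the character and restores input.
; NextLevel opens the next level or prints a win, OutOfLives decrements the level index, and ShowHUD is empty.
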(event Custom|StartLevel
  (bind _returnvalue (Game|GetPlayerController 0))
  (if (Variables|Default|GetInOpening)
    (Variables|Default|SetInOpening false)
    (Variables|/Game/Blueprints/GI_FloorIsLava.GI_FloorIsLava_C|SetGameStarted (Utilities|GetFILGameInstance) true)
    (Game|Player|SetViewTargetwithBlend (Game|GetPlayerController 0) (.Character (Utilities|GetFILCharacter)) 1.5 "VTBlend_Linear" 0.0 false)
    (Utilities|FlowControl|Delay 1.5)
    (Input|EnableInput (Game|GetPlayerCharacter 0) _returnvalue)
    (Variables|/Script/Engine.PlayerController|SetbShowMouseCursor _returnvalue false)))

(event EventBeginPlay
  (bind _returnvalue (Game|GetPlayerController 0))
  (bind _fil_gameinstance (Utilities|GetFILGameInstance))
  (bind _gamestarted (Variables|/Game/Blueprints/GI_FloorIsLava.GI_FloorIsLava_C|GetGameStarted _fil_gameinstance))
  ;[1 1 1] Update max level reached
  (bind _index (CallFunction|GetCurrentLevelIndex))
  (Default|LevelReached (Utilities|GetFILGameInstance) _index)
  (CallFunction|Fadein _gamestarted)
  (if _gamestarted
    _
    (else
      (CallFunction|ShowMainMenu)))
  (Input|DisableInput (Game|GetPlayerCharacter 0) _returnvalue)
  (Variables|/Script/Engine.PlayerController|SetbShowMouseCursor _returnvalue true))

(fn ConstructionScript
  (|CallParentFunction))

(fn OutOfLives
  (bind _fil_gameinstance (Utilities|GetFILGameInstance))
  ;[1 1 1] Decrement current level, don't let it go below 0
  (Variables|/Game/Blueprints/GI_FloorIsLava.GI_FloorIsLava_C|SetCurrentLevel _fil_gameinstance (Math|Integer|Max(Integer) 0 (- (Variables|/Game/Blueprints/GI_FloorIsLava.GI_FloorIsLava_C|GetCurrentLevel _fil_gameinstance) 1))))

(fn ShowMainMenu
  (bind _returnvalue (UserInterface|CreateWidget "/Game/UI/WI_AchievementsMenu.WI_AchievementsMenu_C" (Game|GetPlayerController 0)))
  (UserInterface|Viewport|AddtoViewport _returnvalue 0))

(fn ShowHUD)

(fn Fadein
  (params (ShowLevelName :type Boolean))
  (bind _outactors (Actor|GetAllActorswithTag "OpeningCam"))
  (Game|Player|SetViewTargetwithBlend (Game|GetPlayerController 0) (Utilities|Array|Get(acopy) _outactors) 0.0 "VTBlend_Linear" 0.0 false)
  (if ShowLevelName
    (bind _returnvalue (UserInterface|CreateWidget "/Game/UI/WI_LevelName.WI_LevelName_C"))
    (UserInterface|Viewport|AddtoViewport _returnvalue 0)))

(fn NextLevel
  (bind _fil_gameinstance (Utilities|GetFILGameInstance))
  (bind _levels (Variables|/Game/Blueprints/GI_FloorIsLava.GI_FloorIsLava_C|GetLevels _fil_gameinstance))
  (bind _currentlevel (Variables|/Game/Blueprints/GI_FloorIsLava.GI_FloorIsLava_C|GetCurrentLevel _fil_gameinstance))
  (bind _returnvalue (+ _currentlevel 1))
  (if (== (Utilities|Array|Length _levels) _returnvalue)
    (Development|PrintString "You win!")
    (else
      (Game|OpenLevel(byName) (.levelfilename (Utilities|Array|Get(acopy) _levels _returnvalue))))))