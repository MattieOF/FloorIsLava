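; Game instance for the Floor Is Lava game, holding lives, current level and achievement data.
; On Init it records starting Lives as MaxLives and builds lookup maps from level file name to index and achievement ID to achievement.
; LevelReached sets the current level, and achievements, awarded directly or by name, pop a WI_Achievement widget.
; Earned achievements are not recorded: AwardAchievement and HasAchieved always return false.
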(event EventInit
  ;[1 1 1] Init max lives to initial value of lives
  (Variables|GameState|SetMaxLives (Variables|GameState|GetLives))
  ;[1 1 1] Populate maps
  (CallFunction|PopulateLevelNametoIndexMap)
  (CallFunction|PopulateAchievementNametoRefMap))

(fn PopulateLevelNametoIndexMap
  ;[1 1 1] For each level, add it to the name->index map
  (for (_array_element _array_index) (Variables|Default|GetLevels)
    (Utilities|Map|Add (Variables|Default|GetLevelNameToIndexMap) (.levelfilename _array_element) _array_index)))

(fn LevelReached
  (params (LevelIndex :type Integer))
  (Variables|GameState|SetCurrentLevel LevelIndex))

(fn PopulateAchievementNametoRefMap
  ;[1 1 1] For each achievement, add it to the name->ref map
  (for _array_element (Variables|Default|GetAchievements)
    (Utilities|Map|Add (Variables|Default|GetAchievementNameToRefMap) (.ID (Utilities|Struct|BreakAchievement _array_element)) _array_element)))

(fn AwardAchievement
  (params (Achievement :type Achievement%20Structure))
  ;[1 1 1] Show achievement UI
  (bind _returnvalue (UserInterface|CreateWidget "/Game/UI/WI_Achievement.WI_Achievement_C"))
  (Default|Initialise _returnvalue Achievement)
  (UserInterface|Viewport|AddtoViewport _returnvalue 0)
  (return false))

(fn AwardAchievementfromName
  (params (Name :type Name))
  ;[1 1 1] Get achievement object from name and call AwardAchievement with it
  (bind _alreadyhad (CallFunction|AwardAchievement (.Value (Utilities|Map|Find (Variables|Default|GetAchievementNameToRefMap) Name))))
  (return _alreadyhad))

(fn HasAchieved
  (params (Achievement :type Name))
  (return false))